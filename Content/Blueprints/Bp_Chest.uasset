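; Chest Blueprint that animates its cover by pitching it on timelines, scaled to 60 degrees.
; BeginPlay plays one timeline immediately.
; A custom event checks the Keys array on BP_Player, and any false entry clears CanOpen and plays a second timeline on the same cover.
; The final CanOpen branch has no action when true, so holding all keys triggers nothing further.
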(event Custom|CustomEvent
  (Variables|Default|SetCan_open true)
  (for _array_element (Variables|/Game/BP_Player.BP_Player_C|GetKeys (.AsBP%20Player (Utilities|Casting|CastToBP_Player (Game|GetPlayerCharacter 0))))
    (if (not _array_element)
      (Variables|Default|SetCan_open false)
      (bind _newtrack_0 (Timeline|Timeline_0 Play)
        (:Update
          (Transformation|SetRelativeRotation (Variables|Default|GetChest_cover_StaticMeshComponent0) (Math|Rotator|MakeRotator 0.0 (* _newtrack_0 6e+01) 0.0) false false)))))
  (if (Variables|Default|GetCan_open)
    _))

(event EventBeginPlay
  (bind _newtrack_0 (Timeline|Timeline Play)
    (:Update
      (Transformation|SetRelativeRotation (Variables|Default|GetChest_cover_StaticMeshComponent0) (Math|Rotator|MakeRotator 0.0 (* _newtrack_0 6e+01) 0.0) false false))))

(fn ConstructionScript)