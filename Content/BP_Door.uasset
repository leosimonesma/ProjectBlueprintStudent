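; BP_Door is a double door with custom Open_Door and Close_Door events for other logic to call.
; Each event instantly snaps the two door meshes to fixed, mirrored relative rotations, with closing reversing the signs used for opening.
; A DoorIsOpen flag records the state; the Blueprint has no interpolation, overlap trigger or active tick logic of its own.
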(event Custom|Close_Door
  (Transformation|SetRelativeRotation (Variables|Default|GetDoor_4_StaticMeshComponent0) "0.000000,-80.000000,0.000000" false false)
  (Transformation|SetRelativeRotation (Variables|Default|GetDoor_3_StaticMeshComponent0) "0.000000,80.000000,0.000000" false false)
  (Variables|Default|SetDoor_Is_Open false))

(event Custom|Open_Door
  (Transformation|SetRelativeRotation (Variables|Default|GetDoor_4_StaticMeshComponent0) "0.000000,80.000000,0.000000" false false)
  (Transformation|SetRelativeRotation (Variables|Default|GetDoor_3_StaticMeshComponent0) "0.000000,-80.000000,0.000000" false false)
  (Variables|Default|SetDoor_Is_Open true))

(event EventBeginPlay)

(event Collision|EventActorBeginOverlap
  (params (OtherActor :type Actor%20Object%20Reference)))

(event EventTick
  (params (DeltaSeconds :type Float%20%28single-precision%29)))

(fn ConstructionScript)