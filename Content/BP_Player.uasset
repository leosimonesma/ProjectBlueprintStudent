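; BP_Player is the player Blueprint, handling interaction with doors.
; When IA_Interact starts, it casts player character 0 to BP_Player and runs a short Visibility line trace forward from that player's Camera, with debug drawing.
; If the trace hits a BP_Door, it calls that door's OpenDoor through a direct cast.
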(event Input|EnhancedActionEvents|EnhancedInputActionIA_Interact
  (params (ActionValue :type Boolean) (ElapsedSeconds :type Float%20%28double-precision%29) (TriggeredSeconds :type Float%20%28double-precision%29) (InputAction :type Input%20Action%20Object%20Reference :default "/Game/Inputs/Actions/IA_Interact.IA_Interact"))
  ;[1 1 1] Line trace interact
  (:Started
    (bind _asbp_player (Utilities|Casting|CastToBP_Player (Game|GetPlayerCharacter 0)))
    (bind (_outhit _returnvalue) (Collision|LineTraceByChannel (Transformation|GetWorldLocation (Variables|BP_Player_C|GetCamera _asbp_player)) (+ (Transformation|GetWorldLocation (Variables|BP_Player_C|GetCamera _asbp_player)) (* (Math|Vector|GetForwardVector (Variables|BP_Player_C|GetCamera _asbp_player)) 2e+02)) "TraceTypeQuery1" false 0 "ForDuration"))
    (if _returnvalue
      (bind _asbp_door (Utilities|Casting|CastToBP_Door (.hitactor _outhit)))
      (Default|OpenDoor _asbp_door))))

(event EventBeginPlay)

(event Collision|EventActorBeginOverlap
  (params (OtherActor :type Actor%20Object%20Reference)))

(event EventTick
  (params (DeltaSeconds :type Float%20%28single-precision%29)))

(fn ConstructionScript)